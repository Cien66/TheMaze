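; BP_BoardCharacter is a character that steps field by field across the board from BoardPathCreatorSubsystem, driven by IA_Player input.
; HandleInput shifts row or column, X taking priority over Y, and checks only that the resulting flat index is valid.
; MoveTo locks new targets, then timelines turn the actor toward the field (skipped within tolerance) and slide it there at constant height, unlocking on arrival.
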(event Custom|MoveTo
  (params (TargetLocation :type Board%20Field%20Object%20Reference))
  (Utilities|IsValid TargetLocation
    (:Is%20Valid
      (if (!= TargetLocation (Variables|Default|GetCurrentBoardField))
        (Variables|Default|SetCurrentBoardField TargetLocation)
        (Variables|Default|SetbCanSetNewTarget false)
        (CallFunction|UpdateStartandTargetLocation)
        (CallFunction|RotationtoTarget)))))

(event Custom|RotationToTarget
  (CallFunction|UpdateStartandTargetRotation)
  (if (Utilities|Operators|EqualEqual (Variables|Default|GetStartRotation) (Variables|Default|GetTargetRotaion) 5.0)
    (CallFunction|UpdateLocation)
    (else
      (CallFunction|UpdateRotation))))

(event Custom|UpdateRotation
  (bind _alpha (Timeline|Timeline PlayFromStart)
    (:Update
      (Transformation|SetActorRotation (Math|Rotator|Lerp(Rotator) (Variables|Default|GetStartRotation) (Variables|Default|GetTargetRotaion) _alpha true)))
    (:Finished
      (Transformation|SetActorRotation (Variables|Default|GetTargetRotaion))
      (CallFunction|UpdateLocation))))

(event Custom|UpdateLocation
  (bind _targetlocation (Variables|Default|GetTargetLocation))
  (bind _alpha (Timeline|MovementTimeline PlayFromStart)
    (:Update
      (Transformation|SetActorLocation (Math|Vector|Lerp(Vector) (Variables|Default|GetStartLocation) _targetlocation _alpha) false false))
    (:Finished
      (Transformation|SetActorLocation _targetlocation false false)
      (Variables|Default|SetbCanSetNewTarget true))))

(event Input|EnhancedActionEvents|EnhancedInputActionIA_Player
  (params (ActionValue :type Vector%202D%20Structure) (ElapsedSeconds :type Float%20%28double-precision%29) (TriggeredSeconds :type Float%20%28double-precision%29) (InputAction :type Input%20Action%20Object%20Reference :default "/Game/Inputs/IA_Player.IA_Player"))
  (:Started
    (CallFunction|HandleInput ActionValue)))

(fn ConstructionScript)

(fn UpdateStartandTargetRotation
  (Variables|Default|SetStartRotation (Transformation|GetActorRotation))
  (Variables|Default|SetTargetRotaion (Math|Rotator|FindLookatRotation (Variables|Default|GetStartLocation) (Variables|Default|GetTargetLocation))))

(fn UpdateStartandTargetLocation
  (bind _currentboardfield (Variables|Default|GetCurrentBoardField))
  (bind _returnvalue (Transformation|GetWorldLocation _currentboardfield))
  (Variables|Default|SetTargetLocation (Math|Vector|MakeVector (.x _returnvalue) (.y _returnvalue) (.z (Transformation|GetActorLocation))))
  (Variables|Default|SetStartLocation (Transformation|GetActorLocation)))

(fn HandleInput
  (params (InputVector :type Vector%202D%20Structure))
  (bind (_x _y) (Math|Vector2D|BreakVector2D InputVector))
  (bind _returnvalue (Subsystems|GetBoardPathCreatorSubsystem))
  (bind _returnvalue_2 (Class|BoardPathCreatorSubsystem|GetBoard _returnvalue))
  (bind _returnvalue_3 (Class|Board|GetFields _returnvalue_2))
  (Development|PrintString (Utilities|String|ToString(Vector2d) InputVector) true true "(R=1.000000,G=0.000000,B=0.108605,A=1.000000)" 2e+01)
  (if (Variables|Default|GetbCanSetNewTarget)
    (LocalVariables|SetCurrentRow (.OutRow (Class|Board|CovertIndextoRowandColumn (Class|BoardPathCreatorSubsystem|GetBoard (Subsystems|GetBoardPathCreatorSubsystem)) (Variables|Default|GetCurrentFieldIndex))))
    (LocalVariables|SetCurrentColumn (.OutColumn (Class|Board|CovertIndextoRowandColumn (Class|BoardPathCreatorSubsystem|GetBoard (Subsystems|GetBoardPathCreatorSubsystem)) (Variables|Default|GetCurrentFieldIndex))))
    (Math|Float|CompareFloat _x 0.0
      (:>
        (Math|Integer|IncrementInt (LocalVariables|GetCurrentRow)
          (:%20%20
            _)))
      (:==
        (Math|Float|CompareFloat _y 0.0
          (:>
            (Math|Integer|IncrementInt (LocalVariables|GetCurrentColumn)
              (:%20%20
                _)))
          (:<
            (Math|Integer|DecrementInt (LocalVariables|GetCurrentColumn)
              (:%20%20
                _)))))
      (:<
        (Math|Integer|DecrementInt (LocalVariables|GetCurrentRow)
          (:%20%20
            _))))
    (bind _output_get (LocalVariables|SetIndex (Class|Board|ConvertRowandColumntoIndex _returnvalue_2 (LocalVariables|GetCurrentRow) (LocalVariables|GetCurrentColumn))))
    (if (Utilities|Array|IsValidIndex _returnvalue_3 _output_get)
      (CallFunction|Moveto (Utilities|Array|Get(acopy) _returnvalue_3 _output_get))
      (Variables|Default|SetCurrentFieldIndex (LocalVariables|GetIndex)))))