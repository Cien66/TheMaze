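; Game mode for a board path game in which the fields are shown briefly, then hidden.
; After a timer, it hides every field from the board path creator subsystem's board and gives the player controller its input mapping.
; It binds to the player board checker's goal event; the win function resets input and starts another timer, with a separate function to reopen the gameplay level.
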(event Custom|SetShadowOnBoard
  (bind _returnvalue (Subsystems|GetBoardPathCreatorSubsystem))
  (bind _returnvalue_2 (Class|BoardPathCreatorSubsystem|GetBoard _returnvalue))
  (Utilities|IsValid _returnvalue_2
    (:Is%20Valid
      (for _array_element (Class|Board|GetFields _returnvalue_2)
        (Class|BoardField|SetIsHide _array_element true))
      (bind _asbp_board_player_controller (Utilities|Casting|CastToBP_BoardPlayerController (Game|GetPlayerController 0)))
      (Default|SetInput _asbp_board_player_controller "/Game/Inputs/IMC_Player.IMC_Player"))))

(event EventEndPlay
  (params (EndPlayReason :type EEndPlayReason%20Enum :default "Destroyed"))
  (Utilities|Time|ClearandInvalidateTimerbyHandle (Variables|Default|GetTimer))
  (|CallParentFunction EndPlayReason))

(event EventBeginPlay
  (|CallParentFunction)
  (bind _returnvalue (Utilities|Time|SetTimerbyEvent (delegate Custom|SetShadowOnBoard) (Variables|Default|GetHideTime)))
  (Variables|Default|SetTimer _returnvalue)
  (EventDispatchers|BindEventtoOnPlayeronMeta (Subsystems|GetPlayerBoardCheckerSubsystem) (EventDispatchers|CreateEvent :!event OnPlayerWin)))

(fn ConstructionScript)

(fn OnPlayerWin
  (bind _asbp_board_player_controller (Utilities|Casting|CastToBP_BoardPlayerController (Game|GetPlayerController 0)))
  (Default|SetInput _asbp_board_player_controller)
  (Utilities|Time|SetTimerbyEvent (EventDispatchers|CreateEvent :!event ResetBoardLevel) (Variables|Default|GetHideTime)))

(fn ResetBoardLevel
  (Game|OpenLevel(byObjectReference) "/Game/Maps/M_Gameplay.M_Gameplay"))