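; BP_Board is the game board Blueprint that initializes its fields when play begins.
; On BeginPlay it runs the parent logic, registers the Start field as the safe field with the PlayerBoardCheckerSubsystem, then sets every field to not hidden.
; GetStartField searches the board's fields and returns the first one whose kind is Start.
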(event EventBeginPlay
  (|CallParentFunction)
  (Class|PlayerBoardCheckerSubsystem|SetSafeField (Subsystems|GetPlayerBoardCheckerSubsystem) (CallFunction|GetStartField))
  (for _array_element (Class|Board|GetFields)
    (Class|BoardField|SetIsHide _array_element false)))

(fn ConstructionScript)

(fn GetStartField
  (bind _array_element (Utilities|Array|ForEachLoopwithBreak (Class|Board|GetFields) :!label _label)
    (:LoopBody
      (if (== (Class|BoardField|GetKindOfField _array_element) "(TagName=\"Field.Kind.Start\")")
        (LocalVariables|SetFoundField _array_element)
        (goto _label Break)))
    (:Completed
      (return (LocalVariables|GetFoundField)))))